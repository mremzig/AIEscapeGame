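; BP_Door is an interactable door that stays locked until the level contains no BP_Key actors.
; Tick scans for BP_Key actors every frame and sets HasKey once none remain, inferring pickup from their absence.
; With the key, Interact uses a FlipFlop to play or reverse a timeline that swings the door mesh's yaw by 90 degrees.
; Without it, Interact prints a Turkish message saying a key is needed.
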(event `/Game/Items/BPI_Interact.Interact`
  (if (`self.HasKey?`)
    (`/Engine/EditorBlueprintResources/StandardMacros.FlipFlop`
      (:`A`
        (bind (_direction _door_track) (`Timeline|Door Timeline` :!label _label)
          (:`Update`
            (`SceneComponent.K2_SetRelativeRotation` (`self.SM_Door`) (`KismetMathLibrary.MakeRotator` 0.0 0.0 (`KismetMathLibrary.Lerp` 0.0 -90.0 _door_track)) false false))))
      (:`B`
        (goto _label :!via `Reverse`)))
    (else
      (`KismetSystemLibrary.PrintString` "Kapıyı Açmam İçin Anahtar Lazım!"))))

(event `self.ReceiveTick`
  (params (DeltaSeconds :type "Float (single-precision)"))
  (bind _outactors (`GameplayStatics.GetAllActorsOfClass` "/Game/Items/BP_Key.BP_Key_C"))
  (if (`KismetArrayLibrary.Array_IsEmpty` _outactors)
    (set `self.HasKey?` true)))

(fn `UserConstructionScript`)